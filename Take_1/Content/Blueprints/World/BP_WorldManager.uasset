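; World manager that streams procedural terrain by spawning BP_WorldChunk actors around the player as they move.
; A looping MultiGate on Tick snaps player location to a 1000-unit grid and checks the eight neighbouring cells, excluding the centre.
; IsChunkSpawned linearly searches SpawnedChunks by X/Y.
; Missing cells get a chunk built from GetNoiseForChunk vertices and shared Triangles, then are recorded without ever being removed.
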(event EventBeginPlay
  (Variables|Default|SetAmplitude 50))

(event Collision|EventActorBeginOverlap
  (params (OtherActor :type Actor%20Object%20Reference)))

(event EventTick
  (params (DeltaSeconds :type Float%20%28single-precision%29))
  (bind _returnvalue (Game|GetPlayerCharacter 0))
  (bind _triangles (Variables|Default|GetTriangles))
  (bind _returnvalue_2 (Transformation|GetActorLocation _returnvalue))
  (bind _returnvalue_3 (/ _returnvalue_2 1000))
  (bind _returnvalue_4 (Class|KismetMathLibrary|FTruncVector _returnvalue_3))
  (bind _returnvalue_5 (Math|Conversions|ToVector(Float) _returnvalue_4))
  (bind _return_value (CallFunction|CalculateChunkStartingLocation -1 1 _returnvalue_5))
  (bind _return_value_2 (CallFunction|CalculateChunkStartingLocation 0 1 _returnvalue_5))
  (bind _return_value_3 (CallFunction|CalculateChunkStartingLocation 1 1 _returnvalue_5))
  (bind _return_value_4 (CallFunction|CalculateChunkStartingLocation 1 0 _returnvalue_5))
  (bind _return_value_5 (CallFunction|CalculateChunkStartingLocation 1 -1 _returnvalue_5))
  (bind _return_value_6 (CallFunction|CalculateChunkStartingLocation 0 -1 _returnvalue_5))
  (bind _return_value_7 (CallFunction|CalculateChunkStartingLocation -1 -1 _returnvalue_5))
  (bind _return_value_8 (CallFunction|CalculateChunkStartingLocation -1 0 _returnvalue_5))
  (Utilities|FlowControl|MultiGate false true -1
    (:Out%200
      (Utilities|FlowControl|Sequence
        (:then_0
          (if (not (CallFunction|IsChunkSpawned _return_value_2))
            (bind _returnvalue_6 (Class|WorldManager|GetNoiseforChunk _return_value_2))
            (bind _returnvalue_7 (Game|SpawnActorfromClass "/Game/Blueprints/World/BP_WorldChunk.BP_WorldChunk_C" (Math|Transform|MakeTransform _return_value_2 "0, 0, 0" "1,1,1") "Undefined" 0 _return_value_2 _returnvalue_6 _triangles 0))
            (Transformation|SetMobility (Variables|/Game/Blueprints/World/BP_WorldChunk.BP_WorldChunk_C|GetRuntimeMeshComponentStatic _returnvalue_7) "Stationary")
            (Utilities|Array|Add (Variables|Default|GetSpawnedChunks) _returnvalue_7)))
        (:then_1
          (if (not (CallFunction|IsChunkSpawned _return_value_3))
            (bind _returnvalue_8 (Class|WorldManager|GetNoiseforChunk _return_value_3))
            (bind _returnvalue_9 (Game|SpawnActorfromClass "/Game/Blueprints/World/BP_WorldChunk.BP_WorldChunk_C" (Math|Transform|MakeTransform _return_value_3 "0, 0, 0" "1,1,1") "Undefined" 0 _return_value_3 _returnvalue_8 _triangles 0))
            (Utilities|Array|Add (Variables|Default|GetSpawnedChunks) _returnvalue_9)))
        (:then_2
          (if (not (CallFunction|IsChunkSpawned _return_value_4))
            (bind _returnvalue_10 (Class|WorldManager|GetNoiseforChunk _return_value_4))
            (bind _returnvalue_11 (Game|SpawnActorfromClass "/Game/Blueprints/World/BP_WorldChunk.BP_WorldChunk_C" (Math|Transform|MakeTransform _return_value_4 "0, 0, 0" "1,1,1") "Undefined" 0 _return_value_4 _returnvalue_10 _triangles 0))
            (Utilities|Array|Add (Variables|Default|GetSpawnedChunks) _returnvalue_11)))
        (:then_3
          (if (not (CallFunction|IsChunkSpawned _return_value_5))
            (bind _returnvalue_12 (Class|WorldManager|GetNoiseforChunk _return_value_5))
            (bind _returnvalue_13 (Game|SpawnActorfromClass "/Game/Blueprints/World/BP_WorldChunk.BP_WorldChunk_C" (Math|Transform|MakeTransform _return_value_5 "0, 0, 0" "1,1,1") "Undefined" 0 _return_value_5 _returnvalue_12 _triangles 0))
            (Utilities|Array|Add (Variables|Default|GetSpawnedChunks) _returnvalue_13)))
        (:then_4
          (if (not (CallFunction|IsChunkSpawned _return_value_6))
            (bind _returnvalue_14 (Class|WorldManager|GetNoiseforChunk _return_value_6))
            (bind _returnvalue_15 (Game|SpawnActorfromClass "/Game/Blueprints/World/BP_WorldChunk.BP_WorldChunk_C" (Math|Transform|MakeTransform _return_value_6 "0, 0, 0" "1,1,1") "Undefined" 0 _return_value_6 _returnvalue_14 _triangles 0))
            (Utilities|Array|Add (Variables|Default|GetSpawnedChunks) _returnvalue_15)))
        (:then_5
          (if (not (CallFunction|IsChunkSpawned _return_value_7))
            (bind _returnvalue_16 (Class|WorldManager|GetNoiseforChunk _return_value_7))
            (bind _returnvalue_17 (Game|SpawnActorfromClass "/Game/Blueprints/World/BP_WorldChunk.BP_WorldChunk_C" (Math|Transform|MakeTransform _return_value_7 "0, 0, 0" "1,1,1") "Undefined" 0 _return_value_7 _returnvalue_16 _triangles 0))
            (Utilities|Array|Add (Variables|Default|GetSpawnedChunks) _returnvalue_17)))
        (:then_6
          (if (not (CallFunction|IsChunkSpawned _return_value_8))
            (bind _returnvalue_18 (Class|WorldManager|GetNoiseforChunk _return_value_8))
            (bind _returnvalue_19 (Game|SpawnActorfromClass "/Game/Blueprints/World/BP_WorldChunk.BP_WorldChunk_C" (Math|Transform|MakeTransform _return_value_8 "0, 0, 0" "1,1,1") "Undefined" 0 _return_value_8 _returnvalue_18 _triangles 0))
            (Utilities|Array|Add (Variables|Default|GetSpawnedChunks) _returnvalue_19)))
        (:then_7
          (if (not (CallFunction|IsChunkSpawned _return_value))
            (bind _returnvalue_20 (Class|WorldManager|GetNoiseforChunk _return_value))
            (bind _returnvalue_21 (Game|SpawnActorfromClass "/Game/Blueprints/World/BP_WorldChunk.BP_WorldChunk_C" (Math|Transform|MakeTransform _return_value "0, 0, 0" "1,1,1") "Undefined" 0 _return_value _returnvalue_20 _triangles 0))
            (Utilities|Array|Add (Variables|Default|GetSpawnedChunks) _returnvalue_21)))))))

(fn ConstructionScript)

(fn IsChunkSpawned
  (params (Chunk%20Location :type Vector))
  (for _index (range 0 (- (Utilities|Array|Length (Variables|Default|GetSpawnedChunks)) 1))
    (if (and (== (.x (Variables|/Game/Blueprints/World/BP_WorldChunk.BP_WorldChunk_C|GetStartingLocation (Utilities|Array|Get(acopy) (Variables|Default|GetSpawnedChunks) _index))) (.x Chunk%20Location)) (== (.y (Variables|/Game/Blueprints/World/BP_WorldChunk.BP_WorldChunk_C|GetStartingLocation (Utilities|Array|Get(acopy) (Variables|Default|GetSpawnedChunks) _index))) (.y Chunk%20Location)))
      (return true)))
  (return false))

(fn CalculateChunkStartingLocation
  (params (ChunkLocationOffsetX :type Integer) (ChunkLocationOffsetY :type Integer) (Origin :type Vector))
  (return (* (Math|Vector|MakeVector (+ (.x Origin) (Math|Conversions|ToFloat(Integer) ChunkLocationOffsetX)) (+ (.y Origin) (Math|Conversions|ToFloat(Integer) ChunkLocationOffsetY)) (.z Origin)) 1000)))