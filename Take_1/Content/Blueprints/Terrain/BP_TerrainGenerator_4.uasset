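; Terrain generator that builds a blocky cube landscape in its construction script from fixed-seed FastNoise.
; It samples 2D noise over a square grid, scales it into height, and GetBlockType picks the water, sand, grass, dirt or stone instanced mesh by height band.
; An earlier approach, recursive four-cell random height subdivision feeding BuildTerrainFromHeightData, and a flat-ground builder remain in unconnected nodes; BeginPlay does nothing.
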(event EventBeginPlay)

(fn ConstructionScript
  (bind _cubethickness (Variables|Default|GetCubeThickness))
  (bind _returnvalue (Game|ConstructObjectfromClass "/Script/FastNoiseGenerator.FastNoiseWrapper" self))
  (Class|FastNoiseWrapper|SetupFastNoise _returnvalue "Simplex" 69 0.02 "Quintic" "FBM" 3 2.0 0.5 0.45 "Euclidean" "CellValue")
  (for _index (range 0 200)
    (for _index_2 (range 0 200)
      (bind _returnvalue_2 (Class|FastNoiseWrapper|GetNoise2D _returnvalue (Math|Conversions|ToFloat(Integer) _index) (Math|Conversions|ToFloat(Integer) _index_2)))
      (Components|InstancedStaticMesh|AddInstance (Utilities|Select :Index (CallFunction|GetBlockType (* _cubethickness (* 5 _returnvalue_2))) :Option%200 (Variables|Default|GetInstancedStaticMesh_Water) :Option%201 (Variables|Default|GetInstancedStaticMesh_Sand) :Option%202 (Variables|Default|GetInstancedStaticMesh_Grass) :Option%203 (Variables|Default|GetInstancedStaticMesh_Dirt) :Option%204 (Variables|Default|GetInstancedStaticMesh_Stone)) (Math|Transform|MakeTransform (Math|Vector|MakeVector (* _cubethickness (Math|Conversions|ToFloat(Integer) _index)) (* _cubethickness (Math|Conversions|ToFloat(Integer) _index_2)) (* _cubethickness (* 5 _returnvalue_2))) "0, 0, 0" "1.750000,1.750000,1.750000")))))

(fn CalculateNewCubeLocation
  (params (InPreviousLocation :type Vector))
  (if (<= (.x InPreviousLocation) (.x (Variables|Default|GetBounds_Max)))
    (return (* (Math|Vector|MakeVector (+ (.x InPreviousLocation) 1.0) (.y InPreviousLocation) (.z InPreviousLocation)) 175) false)
    (else
      (return (* (Math|Vector|MakeVector 0.0 (+ (.y InPreviousLocation) 1.0) (+ (.z InPreviousLocation) 1.0)) 175) false))))

(fn IsSatisfied
  (params (CurrentCube :type Vector))
  (return (Class|KismetMathLibrary|EqualExactlyVectorVector CurrentCube (Variables|Default|GetBounds_Max))))

(fn GenerateLevelGround
  (bind _bounds_max (Variables|Default|GetBounds_Max))
  (bind _returnvalue (AddComponent|AddInstancedStaticMeshComponent false))
  (bind _output_get (Variables|Default|SetISM_Level0 _returnvalue))
  (Components|StaticMesh|SetStaticMesh _output_get "/Game/Geometry/Meshes/1M_Cube.1M_Cube")
  (for _index (range 0 (Math|Float|Truncate (.x _bounds_max)))
    (for _index_2 (range 0 (Math|Float|Truncate (.y _bounds_max)))
      (Components|InstancedStaticMesh|AddInstance (Variables|Default|GetISM_Level0) (Math|Transform|MakeTransform (* (Math|Vector|MakeVector (Math|Conversions|ToFloat(Integer) _index) (Math|Conversions|ToFloat(Integer) _index_2) 0.0) (Variables|Default|GetCubeThickness)) "0, 0, 0" "1.750000,1.750000,1.750000")))))

(fn GenerateAverageTerrainLevel
  (params (AverageOfCell :type Integer) (MaxJitter :type Integer))
  (bind _returnvalue (* MaxJitter -1))
  (bind _resultedmap (LocalVariables|GetResultedMap))
  (bind _resultedmap_2 (LocalVariables|GetResultedMap))
  (bind _resultedmap_3 (LocalVariables|GetResultedMap))
  (Utilities|Array|Resize (LocalVariables|GetResultedMap) 0)
  (Utilities|Array|SetArrayElem _resultedmap 0 (Math|Random|RandomIntegerinRange (+ AverageOfCell _returnvalue) (+ AverageOfCell MaxJitter)) true)
  (Utilities|Array|SetArrayElem _resultedmap 3 (Math|Random|RandomIntegerinRange (+ AverageOfCell _returnvalue) (+ AverageOfCell MaxJitter)) true)
  (switch int (Math|Conversions|ToInteger(Boolean) (Math|Random|RandomBool))
    (:0
      (Utilities|Array|SetArrayElem _resultedmap_3 1 (* (Utilities|Array|Get(acopy) _resultedmap_3) -1))
      (Utilities|Array|SetArrayElem _resultedmap_3 2 (* (Utilities|Array|Get(acopy) _resultedmap_3 3) -1)))
    (:1
      (Utilities|Array|SetArrayElem _resultedmap_2 2 (* (Utilities|Array|Get(acopy) _resultedmap_2) -1))
      (Utilities|Array|SetArrayElem _resultedmap_2 1 (* (Utilities|Array|Get(acopy) _resultedmap_2 3) -1))))
  (return (LocalVariables|GetResultedMap)))

(fn BuildTerrainfromHeightData
  (params (HeightData :type Array%20of%20Integers))
  (bind _returnvalue (Utilities|Array|Length HeightData))
  (bind _returnvalue_2 (Math|Conversions|ToFloat(Integer) _returnvalue))
  (bind _returnvalue_3 (Math|Float|Sqrt _returnvalue_2))
  (bind _returnvalue_4 (Math|Float|Truncate _returnvalue_3))
  (bind _returnvalue_5 (AddComponent|AddInstancedStaticMeshComponent false))
  (bind _output_get (Variables|Default|SetISM_Level0 _returnvalue_5))
  (Components|StaticMesh|SetStaticMesh _output_get "/Game/Geometry/Meshes/1M_Cube.1M_Cube")
  (for _index (range 0 _returnvalue_4)
    (for _index_2 (range 0 _returnvalue_4)
      (Components|InstancedStaticMesh|AddInstance (Variables|Default|GetISM_Level0) (Math|Transform|MakeTransform (Math|Vector|MakeVector (Math|Conversions|ToFloat(Integer) (* _index (Variables|Default|GetCubeThickness))) (Math|Conversions|ToFloat(Integer) (* _index_2 (Variables|Default|GetCubeThickness))) (Math|Conversions|ToFloat(Integer) (* (Utilities|Array|Get(acopy) HeightData (+ (* _returnvalue_4 _index) _index_2)) (Variables|Default|GetCubeThickness)))) "0, 0, 0" "1.750000,1.750000,1.750000")))))

(fn GetBlockType
  (params (InLocationZ :type Float%20%28single-precision%29))
  (if (<= InLocationZ 1e+01)
    (return 0)
    (elif (<= InLocationZ 3e+02)
      (return 1)
      (elif (<= InLocationZ 4.5e+02)
        (return 2)
        (elif (<= InLocationZ 6e+02)
          (return 3)
          (else
            (return 4)))))))