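; Terrain generator actor that builds a noise-based heightmap mesh in its construction script.
; Fractal simplex noise sets grid vertex heights, GetBlockType turns height bands into vertex colors, and the triangulated grid becomes a RuntimeMeshComponentStatic section with a ground material.
; A second noise pass is sampled but leaves heights unchanged.
; An older instanced-cube approach using recursive random subdivision remains unwired, and BeginPlay is empty.
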(event EventBeginPlay)

(fn ConstructionScript
  (bind _cubethickness (Variables|Default|GetCubeThickness))
  (bind _runtimemeshcomponentstatic (Variables|Default|GetRuntimeMeshComponentStatic))
  (bind _vertices (Variables|Default|GetVertices))
  (bind _triangles (Variables|Default|GetTriangles))
  (bind _numberofelements (Variables|Default|GetNumberOfElements))
  (bind _numberofelements_2 (Variables|Default|GetNumberOfElements))
  (bind _numberofelements_3 (Variables|Default|GetNumberOfElements))
  (bind _returnvalue (- _numberofelements_2 2))
  (bind _returnvalue_2 (- _numberofelements_3 1))
  (bind _returnvalue_3 (- _numberofelements 1))
  (bind _returnvalue_4 (Game|ConstructObjectfromClass "/Script/FastNoiseGenerator.FastNoiseWrapper" self))
  (Class|FastNoiseWrapper|SetupFastNoise _returnvalue_4 "SimplexFractal" 69 0.02 "Quintic" "FBM" 5 2.0 0.5 0.45 "Euclidean" "CellValue")
  (for _index (range 0 _returnvalue_2)
    (for _index_2 (range 0 _returnvalue_2)
      (bind _returnvalue_5 (Class|FastNoiseWrapper|GetNoise2D _returnvalue_4 (Math|Conversions|ToFloat(Integer) _index) (Math|Conversions|ToFloat(Integer) _index_2)))
      (bind _returnvalue_6 (Utilities|Array|Add (Variables|Default|GetVertices) (Math|Vector|MakeVector (* _cubethickness (Math|Conversions|ToFloat(Integer) _index)) (* _cubethickness (Math|Conversions|ToFloat(Integer) _index_2)) (* _cubethickness (* 10 _returnvalue_5)))))
      (Utilities|Array|SetArrayElem (Variables|Default|GetUV) _returnvalue_6 (Math|Vector2D|MakeVector2D (/ (* _cubethickness (Math|Conversions|ToFloat(Integer) _index)) 1e+03) (/ (* _cubethickness (Math|Conversions|ToFloat(Integer) _index_2)) 1e+03)) true)))
  (bind _returnvalue_7 (Game|ConstructObjectfromClass "/Script/FastNoiseGenerator.FastNoiseWrapper" self))
  (Class|FastNoiseWrapper|SetupFastNoise _returnvalue_7 "Simplex" 169 0.2 "Quintic" "FBM" 3 2.0 0.5 0.45 "Euclidean" "CellValue")
  (for _index_3 (range 0 _returnvalue_3)
    (for _index_4 (range 0 _returnvalue_3)
      (bind _returnvalue_8 (Class|FastNoiseWrapper|GetNoise2D _returnvalue_7 (Math|Conversions|ToFloat(Integer) _index_3) (Math|Conversions|ToFloat(Integer) _index_4)))
      (Utilities|Array|SetArrayElem _vertices (CallFunction|GetFlattenedArrayIndex _index_3 _index_4 _numberofelements) (Math|Vector|MakeVector (.x (Utilities|Array|Get(acopy) _vertices (CallFunction|GetFlattenedArrayIndex _index_3 _index_4 _numberofelements))) (.y (Utilities|Array|Get(acopy) _vertices (CallFunction|GetFlattenedArrayIndex _index_3 _index_4 _numberofelements))) (.z (Utilities|Array|Get(acopy) _vertices (CallFunction|GetFlattenedArrayIndex _index_3 _index_4 _numberofelements)))))
      (Utilities|Array|SetArrayElem (Variables|Default|GetVertexColor) (CallFunction|GetFlattenedArrayIndex _index_3 _index_4 _numberofelements) (.Vertex%20Color (CallFunction|GetBlockType (.z (Utilities|Array|Get(acopy) _vertices (CallFunction|GetFlattenedArrayIndex _index_3 _index_4 _numberofelements))))) true)))
  ;[1 1 1] Calculate Triangles
  (for _index_5 (range 0 _returnvalue)
    (for _index_6 (range 0 _returnvalue)
      (Utilities|Array|Add _triangles (+ _index_6 (* _index_5 _numberofelements_2)))
      (Utilities|Array|Add _triangles (+ (+ _index_6 1) (* _index_5 _numberofelements_2)))
      (Utilities|Array|Add _triangles (+ (+ _index_6 1) (* (+ _index_5 1) _numberofelements_2)))
      (Utilities|Array|Add _triangles (+ _index_6 (* _index_5 _numberofelements_2)))
      (Utilities|Array|Add _triangles (+ (+ _index_6 1) (* (+ _index_5 1) _numberofelements_2)))
      (Utilities|Array|Add _triangles (+ _index_6 (* (+ _index_5 1) _numberofelements_2)))))
  (Class|RuntimeMeshComponentStatic|EnableNormalTangentGeneration _runtimemeshcomponentstatic)
  (Class|RuntimeMeshComponentStatic|CreateSectionfromComponents _runtimemeshcomponentstatic 0 0 0 (Variables|Default|GetVertices) (Variables|Default|GetTriangles) 0 (Variables|Default|GetUV) 0 0 0 (Variables|Default|GetVertexColor) 0 "Infrequent" true)
  (Rendering|Material|SetMaterial _runtimemeshcomponentstatic 0 "/Game/Environment/Materials/M_Terrain_Ground_A_Inst.M_Terrain_Ground_A_Inst"))

(fn CalculateNewCubeLocation
  (params (InPreviousLocation :type Vector))
  (if (<= (.x InPreviousLocation) (.x (Variables|Default|GetBounds_Max)))
    (return (* (Math|Vector|MakeVector (+ (.x InPreviousLocation) 1.0) (.y InPreviousLocation) (.z InPreviousLocation)) 175) false)
    (else
      (return (* (Math|Vector|MakeVector 0.0 (+ (.y InPreviousLocation) 1.0) (+ (.z InPreviousLocation) 1.0)) 175) false))))

(fn IsSatisfied
  (params (CurrentCube :type Vector))
  (return (Class|KismetMathLibrary|EqualExactlyVectorVector CurrentCube (Variables|Default|GetBounds_Max))))

(fn GenerateLevelGround
  (bind _bounds_max (Variables|Default|GetBounds_Max))
  (bind _returnvalue (AddComponent|AddInstancedStaticMeshComponent false))
  (bind _output_get (Variables|Default|SetISM_Level0 _returnvalue))
  (Components|StaticMesh|SetStaticMesh _output_get "/Game/Geometry/Meshes/1M_Cube.1M_Cube")
  (for _index (range 0 (Math|Float|Truncate (.x _bounds_max)))
    (for _index_2 (range 0 (Math|Float|Truncate (.y _bounds_max)))
      (Components|InstancedStaticMesh|AddInstance (Variables|Default|GetISM_Level0) (Math|Transform|MakeTransform (* (Math|Vector|MakeVector (Math|Conversions|ToFloat(Integer) _index) (Math|Conversions|ToFloat(Integer) _index_2) 0.0) (Variables|Default|GetCubeThickness)) "0, 0, 0" "1.750000,1.750000,1.750000")))))

(fn GenerateAverageTerrainLevel
  (params (AverageOfCell :type Integer) (MaxJitter :type Integer))
  (bind _returnvalue (* MaxJitter -1))
  (bind _resultedmap (LocalVariables|GetResultedMap))
  (bind _resultedmap_2 (LocalVariables|GetResultedMap))
  (bind _resultedmap_3 (LocalVariables|GetResultedMap))
  (Utilities|Array|Resize (LocalVariables|GetResultedMap) 0)
  (Utilities|Array|SetArrayElem _resultedmap 0 (Math|Random|RandomIntegerinRange (+ AverageOfCell _returnvalue) (+ AverageOfCell MaxJitter)) true)
  (Utilities|Array|SetArrayElem _resultedmap 3 (Math|Random|RandomIntegerinRange (+ AverageOfCell _returnvalue) (+ AverageOfCell MaxJitter)) true)
  (switch int (Math|Conversions|ToInteger(Boolean) (Math|Random|RandomBool))
    (:0
      (Utilities|Array|SetArrayElem _resultedmap_3 1 (* (Utilities|Array|Get(acopy) _resultedmap_3) -1))
      (Utilities|Array|SetArrayElem _resultedmap_3 2 (* (Utilities|Array|Get(acopy) _resultedmap_3 3) -1)))
    (:1
      (Utilities|Array|SetArrayElem _resultedmap_2 2 (* (Utilities|Array|Get(acopy) _resultedmap_2) -1))
      (Utilities|Array|SetArrayElem _resultedmap_2 1 (* (Utilities|Array|Get(acopy) _resultedmap_2 3) -1))))
  (return (LocalVariables|GetResultedMap)))

(fn BuildTerrainfromHeightData
  (params (HeightData :type Array%20of%20Integers))
  (bind _returnvalue (Utilities|Array|Length HeightData))
  (bind _returnvalue_2 (Math|Conversions|ToFloat(Integer) _returnvalue))
  (bind _returnvalue_3 (Math|Float|Sqrt _returnvalue_2))
  (bind _returnvalue_4 (Math|Float|Truncate _returnvalue_3))
  (bind _returnvalue_5 (AddComponent|AddInstancedStaticMeshComponent false))
  (bind _output_get (Variables|Default|SetISM_Level0 _returnvalue_5))
  (Components|StaticMesh|SetStaticMesh _output_get "/Game/Geometry/Meshes/1M_Cube.1M_Cube")
  (for _index (range 0 _returnvalue_4)
    (for _index_2 (range 0 _returnvalue_4)
      (Components|InstancedStaticMesh|AddInstance (Variables|Default|GetISM_Level0) (Math|Transform|MakeTransform (Math|Vector|MakeVector (Math|Conversions|ToFloat(Integer) (* _index (Variables|Default|GetCubeThickness))) (Math|Conversions|ToFloat(Integer) (* _index_2 (Variables|Default|GetCubeThickness))) (Math|Conversions|ToFloat(Integer) (* (Utilities|Array|Get(acopy) HeightData (+ (* _returnvalue_4 _index) _index_2)) (Variables|Default|GetCubeThickness)))) "0, 0, 0" "1.750000,1.750000,1.750000")))))

(fn GetBlockType
  (params (InLocationZ :type Float%20%28single-precision%29))
  (if (<= InLocationZ -3.5e+02)
    (return 0 "(R=1.000000,G=0.000000,B=0.000000,A=1.000000)")
    (elif (<= InLocationZ 3e+02)
      (return 1 "(R=0.000000,G=1.000000,B=0.000000,A=1.000000)")
      (elif (<= InLocationZ 4.5e+02)
        (return 2 "(R=0.000000,G=0.000000,B=1.000000,A=1.000000)")
        (elif (<= InLocationZ 6e+02)
          (return 3 "(R=1.000000,G=1.000000,B=0.000000,A=1.000000)")
          (else
            (return 4 "(R=1.000000,G=0.000000,B=1.000000,A=1.000000)")))))))

(fn GetFlattenedArrayIndex
  (params (RowIndex :type Integer) (ColumnIndex :type Integer) (MatrixSize :type Integer))
  (return (+ (* RowIndex MatrixSize) ColumnIndex)))