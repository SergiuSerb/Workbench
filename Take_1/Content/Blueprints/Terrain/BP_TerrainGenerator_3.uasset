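; Procedural terrain generator that builds a blocky heightmap from instanced cube meshes in the construction script.
; Five passes expand each height into four: two random values within a shrinking jitter of the parent, plus their negations in randomly swapped slots.
; BuildTerrainFromHeightData reads the flattened result as a square grid, stacking children consecutively rather than as spatial quads.
; BeginPlay is empty, and the flat-ground and cube-location helpers are unused.
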(event EventBeginPlay)

(fn ConstructionScript
  (bind _intermediatearray_2 (Variables|Default|GetIntermediateArray_2))
  (bind _intermediatearray_2_2 (Variables|Default|GetIntermediateArray_2))
  (bind _return_array (CallFunction|GenerateAverageTerrainLevel 0 3))
  (bind _output_get (Variables|Default|SetIntermediateArray_1 _return_array))
  (Utilities|Array|Clear _intermediatearray_2_2)
  (for _array_element _output_get
    (bind _return_array_2 (CallFunction|GenerateAverageTerrainLevel _array_element 2))
    (for _array_element_2 _return_array_2
      (Utilities|Array|Add _intermediatearray_2_2 _array_element_2)))
  (Utilities|Array|Clear (Variables|Default|GetIntermediateArray_1))
  (for _array_element_3 (Variables|Default|GetIntermediateArray_2)
    (bind _return_array_3 (CallFunction|GenerateAverageTerrainLevel _array_element_3 1))
    (for _array_element_4 _return_array_3
      (Utilities|Array|Add (Variables|Default|GetIntermediateArray_1) _array_element_4)))
  (Utilities|Array|Clear _intermediatearray_2)
  (for _array_element_5 (Variables|Default|GetIntermediateArray_1)
    (bind _return_array_4 (CallFunction|GenerateAverageTerrainLevel _array_element_5))
    (for _array_element_6 _return_array_4
      (Utilities|Array|Add _intermediatearray_2 _array_element_6)))
  (Utilities|Array|Clear (Variables|Default|GetIntermediateArray_1))
  (for _array_element_7 (Variables|Default|GetIntermediateArray_2)
    (bind _return_array_5 (CallFunction|GenerateAverageTerrainLevel _array_element_7))
    (for _array_element_8 _return_array_5
      (Utilities|Array|Add (Variables|Default|GetIntermediateArray_1) _array_element_8)))
  (bind _output_get_2 (Variables|Default|SetAverageTerrainLevelOnMap (Variables|Default|GetIntermediateArray_1)))
  (CallFunction|BuildTerrainfromHeightData _output_get_2))

(fn CalculateNewCubeLocation
  (params (InPreviousLocation :type Vector))
  (if (<= (.x InPreviousLocation) (.x (Variables|Default|GetBounds_Max)))
    (return (* (Math|Vector|MakeVector (+ (.x InPreviousLocation) 1.0) (.y InPreviousLocation) (.z InPreviousLocation)) 175) false)
    (else
      (return (* (Math|Vector|MakeVector 0.0 (+ (.y InPreviousLocation) 1.0) (+ (.z InPreviousLocation) 1.0)) 175) false))))

(fn IsSatisfied
  (params (CurrentCube :type Vector))
  (return (Class|KismetMathLibrary|EqualExactlyVectorVector CurrentCube (Variables|Default|GetBounds_Max))))

(fn GenerateLevelGround
  (bind _bounds_max (Variables|Default|GetBounds_Max))
  (bind _returnvalue (AddComponent|AddInstancedStaticMeshComponent false))
  (bind _output_get (Variables|Default|SetISM_Level0 _returnvalue))
  (Components|StaticMesh|SetStaticMesh _output_get "/Game/Geometry/Meshes/1M_Cube.1M_Cube")
  (for _index (range 0 (Math|Float|Truncate (.x _bounds_max)))
    (for _index_2 (range 0 (Math|Float|Truncate (.y _bounds_max)))
      (Components|InstancedStaticMesh|AddInstance (Variables|Default|GetISM_Level0) (Math|Transform|MakeTransform (* (Math|Vector|MakeVector (Math|Conversions|ToFloat(Integer) _index) (Math|Conversions|ToFloat(Integer) _index_2) 0.0) (Variables|Default|GetCubeThickness)) "0, 0, 0" "1.750000,1.750000,1.750000")))))

(fn GenerateAverageTerrainLevel
  (params (AverageOfCell :type Integer) (MaxJitter :type Integer))
  (bind _returnvalue (* MaxJitter -1))
  (bind _resultedmap (LocalVariables|GetResultedMap))
  (bind _resultedmap_2 (LocalVariables|GetResultedMap))
  (bind _resultedmap_3 (LocalVariables|GetResultedMap))
  (Utilities|Array|Resize (LocalVariables|GetResultedMap) 0)
  (Utilities|Array|SetArrayElem _resultedmap 0 (Math|Random|RandomIntegerinRange (+ AverageOfCell _returnvalue) (+ AverageOfCell MaxJitter)) true)
  (Utilities|Array|SetArrayElem _resultedmap 3 (Math|Random|RandomIntegerinRange (+ AverageOfCell _returnvalue) (+ AverageOfCell MaxJitter)) true)
  (switch int (Math|Conversions|ToInteger(Boolean) (Math|Random|RandomBool))
    (:0
      (Utilities|Array|SetArrayElem _resultedmap_3 1 (* (Utilities|Array|Get(acopy) _resultedmap_3) -1))
      (Utilities|Array|SetArrayElem _resultedmap_3 2 (* (Utilities|Array|Get(acopy) _resultedmap_3 3) -1)))
    (:1
      (Utilities|Array|SetArrayElem _resultedmap_2 2 (* (Utilities|Array|Get(acopy) _resultedmap_2) -1))
      (Utilities|Array|SetArrayElem _resultedmap_2 1 (* (Utilities|Array|Get(acopy) _resultedmap_2 3) -1))))
  (return (LocalVariables|GetResultedMap)))

(fn BuildTerrainfromHeightData
  (params (HeightData :type Array%20of%20Integers))
  (bind _returnvalue (Utilities|Array|Length HeightData))
  (bind _returnvalue_2 (Math|Conversions|ToFloat(Integer) _returnvalue))
  (bind _returnvalue_3 (Math|Float|Sqrt _returnvalue_2))
  (bind _returnvalue_4 (Math|Float|Truncate _returnvalue_3))
  (bind _returnvalue_5 (AddComponent|AddInstancedStaticMeshComponent false))
  (bind _output_get (Variables|Default|SetISM_Level0 _returnvalue_5))
  (Components|StaticMesh|SetStaticMesh _output_get "/Game/Geometry/Meshes/1M_Cube.1M_Cube")
  (for _index (range 0 _returnvalue_4)
    (for _index_2 (range 0 _returnvalue_4)
      (Components|InstancedStaticMesh|AddInstance (Variables|Default|GetISM_Level0) (Math|Transform|MakeTransform (Math|Vector|MakeVector (Math|Conversions|ToFloat(Integer) (* _index (Variables|Default|GetCubeThickness))) (Math|Conversions|ToFloat(Integer) (* _index_2 (Variables|Default|GetCubeThickness))) (Math|Conversions|ToFloat(Integer) (* (Utilities|Array|Get(acopy) HeightData (+ (* _returnvalue_4 _index) _index_2)) (Variables|Default|GetCubeThickness)))) "0, 0, 0" "1.750000,1.750000,1.750000")))))