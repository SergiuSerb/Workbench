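; Terrain generator actor that procedurally builds a cluster of cube meshes in its construction script through a bounded random walk.
; Over a fixed loop, CalculateNewCubeLocation derives candidates from the last stored location using per-axis biased steps, with random multipliers that can zero whole coordinates.
; IsValidLocation bounds-checks candidates before cubes are added.
; Random calculations repeat at each use, so checked, stored and placed locations can differ.
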(event EventBeginPlay)

(event Collision|EventActorBeginOverlap
  (params (OtherActor :type Actor%20Object%20Reference)))

(event EventTick
  (params (DeltaSeconds :type Float%20%28single-precision%29)))

(fn ConstructionScript
  (bind _spawnedcubeslocation (Variables|Default|GetSpawnedCubesLocation))
  (bind _returnvalue (Utilities|Array|Length _spawnedcubeslocation))
  (bind _returnvalue_2 (- _returnvalue 1))
  (bind _output (Utilities|Array|Get(acopy) _spawnedcubeslocation _returnvalue_2))
  (bind (_outlocation _bhassucceded) (CallFunction|CalculateNewCubeLocation _output))
  (for _index (range 0 50)
    (if (and _bhassucceded (CallFunction|IsValidLocation _outlocation))
      (Utilities|Array|Add (Variables|Default|GetSpawnedCubesLocation) _outlocation)
      (bind _returnvalue_3 (AddComponent|AddStaticMeshComponent false (Math|Transform|MakeTransform _outlocation "0, 0, 0" "1.750000,1.750000,1.750000")))
      (Utilities|Array|Add (Variables|Default|GetSpawnedCubesInfo) _returnvalue_3)
      (Components|StaticMesh|SetStaticMesh _returnvalue_3 "/Game/Geometry/Meshes/1M_Cube.1M_Cube"))))

(fn CalculateNewCubeLocation
  (params (InPreviousLocation :type Vector))
  (bind _returnvalue (Math|Random|RandomIntegerinRange 0 1))
  (bind _returnvalue_2 (Math|Random|RandomIntegerinRange 0 1))
  (bind _returnvalue_3 (Math|Random|RandomIntegerinRange 0 1))
  (bind _returnvalue_4 (Math|Random|RandomFloatinRange 0.0 1.0))
  (bind _returnvalue_5 (Math|Random|RandomFloatinRange 0.0 1.0))
  (bind _returnvalue_6 (Math|Random|RandomFloatinRange 0.0 1.0))
  (bind _bias_z (Variables|Default|GetBias_Z))
  (bind _bias_x (Variables|Default|GetBias_X))
  (bind _bias_y (Variables|Default|GetBias_Y))
  (bind _cubethickness (Variables|Default|GetCubeThickness))
  (bind _cubethickness_2 (Variables|Default|GetCubeThickness))
  (bind _cubethickness_3 (Variables|Default|GetCubeThickness))
  (bind _returnvalue_7 (>= _returnvalue_4 _bias_z))
  (bind _returnvalue_8 (>= _returnvalue_5 _bias_x))
  (bind _returnvalue_9 (>= _returnvalue_6 _bias_y))
  (bind _returnvalue_10 (select _returnvalue_7 1 -1))
  (bind _returnvalue_11 (select _returnvalue_8 1 -1))
  (bind _returnvalue_12 (select _returnvalue_9 1 -1))
  (bind _returnvalue_13 (* _returnvalue_10 _cubethickness))
  (bind _returnvalue_14 (* _returnvalue_11 _cubethickness_2))
  (bind _returnvalue_15 (* _returnvalue_12 _cubethickness_3))
  (bind _returnvalue_16 (Math|Conversions|ToFloat(Integer) _returnvalue_13))
  (bind _returnvalue_17 (Math|Conversions|ToFloat(Integer) _returnvalue_14))
  (bind _returnvalue_18 (Math|Conversions|ToFloat(Integer) _returnvalue_15))
  (bind _returnvalue_19 (+ (.z InPreviousLocation) _returnvalue_16))
  (bind _returnvalue_20 (+ (.x InPreviousLocation) _returnvalue_17))
  (bind _returnvalue_21 (+ (.y InPreviousLocation) _returnvalue_18))
  (bind _returnvalue_22 (* _returnvalue _returnvalue_19))
  (bind _returnvalue_23 (* _returnvalue_2 _returnvalue_20))
  (bind _returnvalue_24 (* _returnvalue_3 _returnvalue_21))
  (bind _returnvalue_25 (Math|Vector|MakeVector _returnvalue_23 _returnvalue_24 _returnvalue_22))
  (if (Math|Vector|Equal(Vector) _returnvalue_25 (Math|Vector|MakeVector (.x InPreviousLocation) (.y InPreviousLocation) (.z InPreviousLocation)) 0.0001)
    (return _returnvalue_25 false)
    (else
      (return _returnvalue_25 true))))

(fn IsValidLocation
  (params (InLocation :type Vector))
  (bind _bounds_min (Variables|Default|GetBounds_Min))
  (bind _bounds_max (Variables|Default|GetBounds_Max))
  (if (and (Math|Boolean|ANDBoolean (>= (.x InLocation) (.x _bounds_min)) (>= (.y InLocation) (.y _bounds_min)) (>= (.z InLocation) (.z _bounds_min))) (Math|Boolean|ANDBoolean (>= (.x _bounds_max) (.x InLocation)) (>= (.y _bounds_max) (.y InLocation)) (>= (.z _bounds_max) (.z InLocation))))
    (return true)
    (else
      (return true))))