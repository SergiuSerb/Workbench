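; BP_TerrainGenerator_2 is a terrain generator that builds a field of instanced cube meshes at construction time.
; Its Construction Script loops over BoundsMax X and Y, adding scaled instances on a skewed grid spaced by CubeThickness, with Y and Z derived from both indices.
; Helpers for stepping cube locations, testing bounds and filling surrounding space are uncalled.
; The fill helper is unfinished, with an empty while loop that never decrements.
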(event EventBeginPlay)

(fn ConstructionScript
  (bind _bounds_max (Variables|Default|GetBounds_Max))
  (for _index (range 0 (Math|Float|Truncate (.x _bounds_max)))
    (for _index_2 (range 0 (Math|Float|Truncate (.y _bounds_max)))
      (Components|InstancedStaticMesh|AddInstance (Variables|Default|GetInstancedStaticMesh) (Math|Transform|MakeTransform (* (Math|Vector|MakeVector (Math|Conversions|ToFloat(Integer) (* _index -1)) (+ (Math|Conversions|ToFloat(Integer) (* _index_2 -1)) (Math|Conversions|ToFloat(Integer) _index)) (Math|Conversions|ToFloat(Integer) (* _index_2 -1))) (Variables|Default|GetCubeThickness)) "0, 0, 0" "1.750000,1.750000,1.750000")))))

(fn CalculateNewCubeLocation
  (params (InPreviousLocation :type Vector))
  (if (<= (.x InPreviousLocation) (.x (Variables|Default|GetBounds_Max)))
    (return (* (Math|Vector|MakeVector (+ (.x InPreviousLocation) 1.0) (.y InPreviousLocation) (.z InPreviousLocation)) 175) false)
    (else
      (return (* (Math|Vector|MakeVector 0.0 (+ (.y InPreviousLocation) 1.0) (+ (.z InPreviousLocation) 1.0)) 175) false))))

(fn IsSatisfied
  (params (CurrentCube :type Vector))
  (return (Class|KismetMathLibrary|EqualExactlyVectorVector CurrentCube (Variables|Default|GetBounds_Max))))

(fn FillSpaceSurroundingCube
  (params (CubeToSurround :type Vector) (CubesToAdd_XY :type Integer) (CubesToAdd_XZ :type Integer) (CubesToAddYZ :type Integer))
  (bind _output_get (LocalVariables|SetCubesToAddXY_Local CubesToAdd_XY))
  (LocalVariables|SetCubesToAddXZ_Local CubesToAdd_XZ)
  (LocalVariables|SetCubesToAddYZ_Local CubesToAddYZ)
  (AddComponent|AddInstancedStaticMeshComponent false (Math|Transform|MakeTransform (* CubeToSurround (Variables|Default|GetCubeThickness)) "0, 0, 0" "1,1,1"))
  (Utilities|FlowControl|Sequence
    (:then_0
      (while (!= _output_get 0)
        _))))